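; Player actor for an obstacle runner, pushed forward automatically by physics impulses and steered sideways by the MoveRight axis.
; Forward and side impulses scale with mass and frame time, with only the side impulse applied as a velocity change.
; Hitting an obstacle or falling below a height threshold ends the game through BP_GameMode, while overlapping an end point completes the level.
; BeginPlay creates the HUD and caches the game mode.
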(event `self.ReceiveBeginPlay`
  (bind _returnvalue (`|CreateWidget` "/Game/Blueprints/WBP_HUD.WBP_HUD_C"))
  (bind _output_get (set `self.BPW_HUD` _returnvalue))
  (`UserWidget.AddToViewport` _output_get 0)
  (bind _asbp_game_mode (cast `/Game/Blueprints/BP_Only/BP_GameMode` (`GameplayStatics.GetGameMode`)))
  (set `self.BP_GameMode` _asbp_game_mode))

(event `self.ReceiveTick`
  (params (DeltaSeconds :type "Float (single-precision)"))
  (bind (_returnvalue_x _returnvalue_y _returnvalue_z) (`KismetMathLibrary.BreakVector` (`self.K2_GetActorLocation`)))
  (bind _output_get (set `self.DeltaSeconds` DeltaSeconds))
  (if (not (`self.bGameEnded`))
    (`PrimitiveComponent.AddImpulse` (`self.Player`) (`KismetMathLibrary.MakeVector` (* _output_get (* (`PrimitiveComponent.GetMass` (`self.Player`)) (`self.ForwardForce`)))) "None" false)
    (if (< _returnvalue_z -30.0)
      (`self.GameEnded`))))

(event `InputAxis|MoveRight`
  (params (AxisValue :type "Float (single-precision)"))
  (if (not (`self.bGameEnded`))
    (`PrimitiveComponent.AddImpulse` (`self.Player`) (`KismetMathLibrary.MakeVector` 0.0 (* AxisValue (* (* (`PrimitiveComponent.GetMass` (`self.Player`)) (`self.SideForce`)) (`self.DeltaSeconds`)))) "None" true)))

(event `self.Player.OnComponentHit`
  (params (HitComponent :type "PrimitiveComponent Object Reference") (OtherActor :type "Actor Object Reference") (OtherComp :type "PrimitiveComponent Object Reference") (NormalImpulse :type "Vector Structure") (Hit :type "HitResult Structure (by ref)"))
  (cast `/Game/Blueprints/BP_Only/BP_Obstacle` OtherActor)
  (`self.GameEnded`))

(event `self.Player.OnComponentBeginOverlap`
  (params (OverlappedComponent :type "PrimitiveComponent Object Reference") (OtherActor :type "Actor Object Reference") (OtherComp :type "PrimitiveComponent Object Reference") (OtherBodyIndex :type Integer) (bFromSweep :type Boolean) (SweepResult :type "HitResult Structure (by ref)"))
  (cast `/Game/Blueprints/BP_Only/BP_EndPoint` OtherActor)
  (set `self.bGameEnded` true)
  (`/Game/Blueprints/BP_Only/BP_GameMode.LevelComplete` (`self.BP_GameMode`)))

(fn `GameEnded`
  (if (not (`self.bGameEnded`))
    (set `self.bGameEnded` true)
    (`/Game/Blueprints/BP_Only/BP_GameMode.EndGame` (`self.BP_GameMode`))))

(fn `UserConstructionScript`)